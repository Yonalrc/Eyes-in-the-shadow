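; BP_MainMenuMode is a mode Blueprint, filed under Main-menu, that respawns the first-person player character after it is destroyed.
; On BeginPlay it binds to the OnDestroyed event of player 0's BP_FirstPersonCharacter.
; When that fires, it waits briefly, spawns a replacement at the SpawnTransform variable and has player controller 0 possess it.
; It then calls Respawn to rebind the event on the new character, so the cycle repeats.
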(event `Respawn`
  (bind _asbp_first_person_character (cast `/Game/FirstPerson/Blueprints/BP_FirstPersonCharacter` (`GameplayStatics.GetPlayerCharacter` 0) :!label _label))
  (add `self.OnDestroyed` _asbp_first_person_character (delegate `OnDestroyed_`)))

(event `self.ReceiveBeginPlay`
  (goto _label))

(event `OnDestroyed_` :!signature `self.OnDestroyed`
  (params (DestroyedActor :type "Actor Object Reference"))
  (`KismetSystemLibrary.Delay` 2.0)
  (bind _returnvalue (`|SpawnActorFromClass` "/Game/FirstPerson/Blueprints/BP_FirstPersonCharacter.BP_FirstPersonCharacter_C" (`self.Spawn Transform`) "Undefined" "MultiplyWithRoot" null null))
  (`Controller.Possess` (`GameplayStatics.GetPlayerController` 0) _returnvalue)
  (`self.Respawn`))

(fn `UserConstructionScript`)
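; A combination-lock tumbler actor that spins its mesh in pitch and tracks the digit it lands on.
; The G and T debug keys drive forward and inverse Timeline spins, each guarded by a DoOnce that resets on finish.
; NumberCheck maps rotation in 36-degree steps to digits and prints the result.
; The inverse spin zeroes the stored rotation instead of decrementing it, and the BeginPlay randomization calls an empty function.
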(event `ShowTumblerNumber`
  (`KismetSystemLibrary.PrintString` (`KismetStringLibrary.Concat_StrStr` "Tumbler Number:" (`KismetStringLibrary.Conv_IntToString` (`self.TumblerNumber`)))))

(event `Key|T`
  (params (Key :type "Key Structure"))
  (:`Pressed`
    (`self.SpinTrumbleInverse`)))

(event `Key|G`
  (params (Key :type "Key Structure"))
  (:`Pressed`
    (`self.SpinTumbler`)))

(event `self.ReceiveBeginPlay`
  (if (`self.RandomizeRotation?`)
    (`self.RandomizeTumbler`)))

(event `SpinTumbler`
  (`/Engine/EditorBlueprintResources/StandardMacros.DoOnce` false :!label _label
    (:`Completed`
      (bind (_direction _alpha) (`Timeline|Timeline` :!via `PlayFromStart`)
        (:`Update`
          (bind _returnvalue (+ (`self.TumblerRotation`) _alpha))
          (`SceneComponent.K2_SetRelativeRotation` (`self.lockTumbler`) (`KismetMathLibrary.MakeRotator` 0.0 _returnvalue) false false))
        (:`Finished`
          (set `self.TumblerRotation` _returnvalue)
          (`self.NumberCheck`)
          (`self.ShowTumblerNumber`)
          (`self.SpinTumblerReset`)
          (if (>= (`self.TumblerRotation`) 360.0)
            (set `self.TumblerRotation` 0.0)))))))

(event `SpinTumblerReset`
  (goto _label :!via `Reset`))

(event `SpinTrumbleInverse`
  (`/Engine/EditorBlueprintResources/StandardMacros.DoOnce` false :!label _label_2
    (:`Completed`
      (bind (_direction _alpha) (`Timeline|Timeline_0`)
        (:`Update`
          (`SceneComponent.K2_SetRelativeRotation` (`self.lockTumbler`) (`KismetMathLibrary.MakeRotator` 0.0 (- (`self.TumblerRotation`) _alpha)) false false))
        (:`Finished`
          (set `self.TumblerRotation` 0.0)
          (`self.NumberCheck`)
          (`self.ShowTumblerNumber`)
          (`self.SpinTrumbleResetInverse`)
          (if (<= (`self.TumblerRotation`) 360.0)
            (set `self.TumblerRotation` 0.0)))))))

(event `SpinTrumbleResetInverse`
  (goto _label_2 :!via `Reset`))

(fn `NumberCheck`
  (if (== (`KismetMathLibrary.FTrunc` (`self.TumblerRotation`)) 36)
    (set `self.TumblerNumber` 1)
    (elif (== (`KismetMathLibrary.FTrunc` (`self.TumblerRotation`)) 72)
      (set `self.TumblerNumber` 2)
      (elif (== (`KismetMathLibrary.FTrunc` (`self.TumblerRotation`)) 108)
        (set `self.TumblerNumber` 3)
        (elif (== (`KismetMathLibrary.FTrunc` (`self.TumblerRotation`)) 144)
          (set `self.TumblerNumber` 4)
          (elif (== (`KismetMathLibrary.FTrunc` (`self.TumblerRotation`)) 180)
            (set `self.TumblerNumber` 5)
            (elif (== (`KismetMathLibrary.FTrunc` (`self.TumblerRotation`)) 216)
              (set `self.TumblerNumber` 6)
              (elif (== (`KismetMathLibrary.FTrunc` (`self.TumblerRotation`)) 252)
                (set `self.TumblerNumber` 7)
                (elif (== (`KismetMathLibrary.FTrunc` (`self.TumblerRotation`)) 288)
                  (set `self.TumblerNumber` 8)
                  (elif (== (`KismetMathLibrary.FTrunc` (`self.TumblerRotation`)) 324)
                    (set `self.TumblerNumber` 9)
                    (elif (== (`KismetMathLibrary.FTrunc` (`self.TumblerRotation`)) 360)
                      (set `self.TumblerNumber` 0))))))))))))

(fn `RandomizeTumbler`)

(fn `UserConstructionScript`)
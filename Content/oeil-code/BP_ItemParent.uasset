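; Base item actor the player can pick up, inspect in front of the camera, and drop.
; Interacting attaches it to the character's grip with physics and collision off, or starts inspection if the character already holds an object.
; Inspection moves input from character to item: left-drag yaws it, the wheel steps its camera distance, and closing resets its relative transform and unpauses.
; DropItem detaches it ahead of the camera and restores physics.
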(event `InputAction|ouvrir item`
  (params (Key :type "Key Structure")))

(event `InputAction|fermer item` :paused true
  (params (Key :type "Key Structure"))
  (:`Pressed`
    (`self.StopInspect`)
    (`GameplayStatics.SetGamePaused` false)))

(event `/Game/FirstPerson/Blueprints/InteractInterface.LookAt`
  (params (`Player Character` :type "/Game/FirstPerson/Blueprints/BP_FirstPersonCharacter Object Reference")))

(event `/Game/FirstPerson/Blueprints/InteractInterface.InteractWith`
  (params (PlayerCharacter :type "/Game/FirstPerson/Blueprints/BP_FirstPersonCharacter Object Reference"))
  (bind _output_get (set `self.Player Character` PlayerCharacter))
  (`/Game/FirstPerson/Blueprints/BP_FirstPersonCharacter.ObjetTenu` _output_get
    (:`then`
      (`self.StartInspect`))
    (:`else`
      (`self.PickUpItem`))))

(event `Key|LeftMouseButton` :paused true
  (params (Key :type "Key Structure"))
  (:`Pressed`
    (set `self.isRotating?` true))
  (:`Released`
    (set `self.isRotating?` false)))

(event `InputAxisKey|MouseX` :paused true
  (params (AxisValue :type "Float (single-precision)"))
  (if (`self.isRotating?`)
    (`self.K2_SetActorRotation` (`KismetMathLibrary.ComposeRotators` (`self.K2_GetActorRotation`) (`KismetMathLibrary.MakeRotator` 0.0 0.0 (* AxisValue -5.0))))))

(event `InputAxisKey|MouseY` :paused true
  (params (AxisValue :type "Float (single-precision)")))

(event `Key|MouseScrollUp` :paused true
  (params (Key :type "Key Structure"))
  (bind _returnvalue (`GameplayStatics.GetPlayerCameraManager` 0))
  (:`Pressed`
    (bind _output_get (set `self.ZoomLevel` (`KismetMathLibrary.Clamp` (+ (`self.ZoomLevel`) 1) 1 20)))
    (if (< _output_get 20)
      (`self.K2_SetActorLocation` (+ (`PlayerCameraManager.GetCameraLocation` _returnvalue) (* (`KismetMathLibrary.GetForwardVector` (`PlayerCameraManager.GetCameraRotation` _returnvalue)) (* (`self.ZoomLevel`) 20.0)))))))

(event `Key|MouseScrollDown`
  (params (Key :type "Key Structure"))
  (bind _returnvalue (`GameplayStatics.GetPlayerCameraManager` 0))
  (:`Pressed`
    (bind _output_get (set `self.ZoomLevel` (`KismetMathLibrary.Clamp` (- (`self.ZoomLevel`) 1) 1 20)))
    (if (> _output_get 1)
      (`self.K2_SetActorLocation` (+ (`PlayerCameraManager.GetCameraLocation` _returnvalue) (* (`KismetMathLibrary.GetForwardVector` (`PlayerCameraManager.GetCameraRotation` _returnvalue)) (* (`self.ZoomLevel`) 20.0)))))))

(fn `DropItem`
  (bind _returnvalue (`GameplayStatics.GetPlayerCameraManager` 0))
  (bind _staticmesh (`self.StaticMesh`))
  (`self.K2_DetachFromActor` "KeepWorld" "KeepWorld" "KeepWorld")
  (`self.K2_SetActorLocation` (+ (`PlayerCameraManager.GetCameraLocation` _returnvalue) (* (`KismetMathLibrary.GetForwardVector` (`PlayerCameraManager.GetCameraRotation` _returnvalue)) 100.0)))
  (`PrimitiveComponent.SetSimulatePhysics` _staticmesh true)
  (`PrimitiveComponent.SetCollisionEnabled` _staticmesh "QueryAndPhysics"))

(fn `PickUpItem`
  (`self.K2_AttachToComponent` (`/Game/FirstPerson/Blueprints/BP_FirstPersonCharacter.GripItem` (`self.Player Character`)) "None" "SnapToTarget" "SnapToTarget" "KeepRelative")
  (`PrimitiveComponent.SetSimulatePhysics` (`self.StaticMesh`) false)
  (`PrimitiveComponent.SetCollisionEnabled` (`self.StaticMesh`) "NoCollision")
  (set `/Game/FirstPerson/Blueprints/BP_FirstPersonCharacter.ObjetTenu` self (`self.Player Character`)))

(fn `StartInspect`
  (bind _returnvalue (`GameplayStatics.GetPlayerController` 0))
  (bind _returnvalue_2 (`GameplayStatics.GetPlayerCameraManager` 0))
  (bind (_returnvalue_x _returnvalue_y _returnvalue_z) (`KismetMathLibrary.BreakVector` (+ (`PlayerCameraManager.GetCameraLocation` _returnvalue_2) (* (`KismetMathLibrary.GetForwardVector` (`PlayerCameraManager.GetCameraRotation` _returnvalue_2)) 50.0))))
  (`self.DisableInput` (`self.Player Character`) _returnvalue)
  (`self.EnableInput` _returnvalue)
  (`self.K2_SetActorLocation` (`KismetMathLibrary.MakeVector` _returnvalue_x _returnvalue_y (- _returnvalue_z 50.0))))

(fn `StopInspect`
  (bind _returnvalue (`GameplayStatics.GetPlayerController` 0))
  (`self.DisableInput` _returnvalue)
  (`self.EnableInput` (`self.Player Character`) _returnvalue)
  (`self.K2_SetActorRelativeLocation` (0.0 0.0 0.0))
  (`self.K2_SetActorRelativeRotation` (struct)))

(fn `UserConstructionScript`)
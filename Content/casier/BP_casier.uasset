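; Locker the first-person player can hide in and leave with the "se cacher" input.
; Box overlap enables the locker's input and opens a gate; leaving disables both.
; The input toggles player visibility and collision, blends the view between character and locker, and plays a timeline door swing.
; While hidden, a self-recalling delay loop rotates the locker camera from clamped mouse axes, which otherwise pass to the character as pitch input.
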(event `InputAction|se cacher`
  (params (Key :type "Key Structure"))
  ;[1 1 1] Sortir et Rentrer dans le casier
  (:`Pressed`
    (`/Engine/EditorBlueprintResources/StandardMacros.Gate` true :!label _label
      (:`Exit`
        (`|ExecutionSequence`
          (:`then_0`
            (`self.toggleHide`)
            (`self.TournerCamera`)
            (`KismetSystemLibrary.Delay` 0.2)
            (`self.EnableInput` (`GameplayStatics.GetPlayerController` 0) :!label _label_2)
            (goto _label :!via `Open`))
          (:`then_1`
            (bind (_direction _newtrack_0) (`Timeline|OpenCloseDoor` :!via `PlayFromStart`)
              (:`Update`
                (`SceneComponent.K2_SetRelativeRotation` (`self.porte-casier`) (`KismetMathLibrary.MakeRotator` 0.0 0.0 (`KismetMathLibrary.Lerp` (`self.CloseAngle`) (`self.OpenAngle`) _newtrack_0)) false false)))))))))

(event `self.Box.OnComponentBeginOverlap`
  (params (OverlappedComponent :type "PrimitiveComponent Object Reference") (OtherActor :type "Actor Object Reference") (OtherComp :type "PrimitiveComponent Object Reference") (OtherBodyIndex :type Integer) (bFromSweep :type Boolean) (SweepResult :type "HitResult Structure (by ref)"))
  ;[1 1 1] Sortir et Rentrer dans le casier
  (bind _asbp_first_person_character (cast `/Game/FirstPerson/Blueprints/BP_FirstPersonCharacter` OtherActor))
  (set `self.Char ref` _asbp_first_person_character)
  (goto _label_2))

(event `self.Box.OnComponentEndOverlap`
  (params (OverlappedComponent :type "PrimitiveComponent Object Reference") (OtherActor :type "Actor Object Reference") (OtherComp :type "PrimitiveComponent Object Reference") (OtherBodyIndex :type Integer))
  ;[1 1 1] Sortir et Rentrer dans le casier
  (cast `/Game/FirstPerson/Blueprints/BP_FirstPersonCharacter` OtherActor)
  (`self.DisableInput` (`GameplayStatics.GetPlayerController` 0))
  (goto _label :!via `Close`))

(event `TournerCamera`
  ;[1 1 1] Tourner Caméra
  (if (`self.isHiding`)
    (`SceneComponent.K2_SetRelativeRotation` (`self.Camera`) (`KismetMathLibrary.MakeRotator` 0.0 (* (stale `InputAxis|Look Up / Down Mouse` _output_get) -1.0) (stale `InputAxis|Turn Right / Left Mouse` _output_get)) false false)
    (`KismetSystemLibrary.Delay` 0.001)
    (`self.TournerCamera`)))

(event `InputAxis|Look Up / Down Mouse`
  (params (AxisValue :type "Float (single-precision)"))
  ;[1 1 1] Tourner Caméra
  (if (`self.isHiding`)
    (bind _output_get (set `self.Pitch` (`KismetMathLibrary.FClamp` (+ (`self.Pitch`) AxisValue) -40.0 20.0)))
    (else
      (`Pawn.AddControllerPitchInput` (`self.Char ref`) AxisValue))))

(event `InputAxis|Turn Right / Left Mouse`
  (params (AxisValue :type "Float (single-precision)"))
  ;[1 1 1] Tourner Caméra
  (if (`self.isHiding`)
    (bind _output_get (set `self.Yaw` (`KismetMathLibrary.FClamp` (+ (`self.Yaw`) AxisValue) -60.0 60.0)))
    (else
      (`Pawn.AddControllerPitchInput` (`self.Char ref`) AxisValue))))

(fn `toggleHide`
  (bind _returnvalue (`GameplayStatics.GetPlayerController` 0))
  (bind _char_ref (`self.Char ref`))
  (if (`self.isHiding`)
    (set `self.isHiding` false)
    (`self.SetActorHiddenInGame` _char_ref false)
    (`self.SetActorEnableCollision` _char_ref true)
    (`PlayerController.SetViewTargetWithBlend` _returnvalue _char_ref 0.8 "VTBlend_Linear" 0.0 false)
    (else
      (set `self.isHiding` true)
      (`self.SetActorHiddenInGame` _char_ref true)
      (`self.SetActorEnableCollision` _char_ref false)
      (`PlayerController.SetViewTargetWithBlend` _returnvalue self 0.8 "VTBlend_Linear" 0.0 false))))

(fn `UserConstructionScript`)
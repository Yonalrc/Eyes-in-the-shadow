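; Table hiding spot that lets the first-person character hide and watch from the table's own camera.
; Box overlap enables the actor's input and opens a gate, so the "se cacher" action toggles the character's Secacher/Passecacher and blends the view to the table on hiding.
; While hidden, mouse axes feed clamped camera rotation through a self-recalling Delay loop; otherwise they pass through to the character.
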(event `InputAction|se cacher`
  (params (Key :type "Key Structure"))
  (bind _charref (`self.CharRef`))
  (:`Pressed`
    (`/Engine/EditorBlueprintResources/StandardMacros.Gate` true :!label _label
      (:`Exit`
        (if (`/Game/FirstPerson/Blueprints/BP_FirstPersonCharacter.isHiding?` _charref)
          (`/Game/FirstPerson/Blueprints/BP_FirstPersonCharacter.passecacher` _charref)
          (else
            (`/Game/FirstPerson/Blueprints/BP_FirstPersonCharacter.secacher` _charref)
            (`|ExecutionSequence`
              (:`then_0`
                (`PlayerController.SetViewTargetWithBlend` (`GameplayStatics.GetPlayerController` 0) self 0.5 "VTBlend_Linear" 0.0 false)
                (`self.MoveCamera`))
              (:`then_1`
                (`KismetSystemLibrary.Delay` 0.2)
                (`self.EnableInput` (`GameplayStatics.GetPlayerController` 0) :!label _label_2)
                (goto _label :!via `Open`)))))))))

(event `self.Box.OnComponentBeginOverlap`
  (params (OverlappedComponent :type "PrimitiveComponent Object Reference") (OtherActor :type "Actor Object Reference") (OtherComp :type "PrimitiveComponent Object Reference") (OtherBodyIndex :type Integer) (bFromSweep :type Boolean) (SweepResult :type "HitResult Structure (by ref)"))
  (bind _asbp_first_person_character (cast `/Game/FirstPerson/Blueprints/BP_FirstPersonCharacter` OtherActor))
  (set `self.CharRef` _asbp_first_person_character)
  (goto _label_2))

(event `self.Box.OnComponentEndOverlap`
  (params (OverlappedComponent :type "PrimitiveComponent Object Reference") (OtherActor :type "Actor Object Reference") (OtherComp :type "PrimitiveComponent Object Reference") (OtherBodyIndex :type Integer))
  (cast `/Game/FirstPerson/Blueprints/BP_FirstPersonCharacter` OtherActor)
  (`self.DisableInput` (`GameplayStatics.GetPlayerController` 0))
  (goto _label :!via `Close`))

(event `MoveCamera`
  (if (`/Game/FirstPerson/Blueprints/BP_FirstPersonCharacter.isHiding?` (`self.CharRef`))
    (`SceneComponent.K2_SetRelativeRotation` (`self.Camera`) (`KismetMathLibrary.MakeRotator` 0.0 (`KismetMathLibrary.FClamp` (* (stale `InputAxis|Look Up / Down Mouse` _output_get) -1.0) -30.0 30.0) (`KismetMathLibrary.FClamp` (stale `InputAxis|Turn Right / Left Mouse` _output_get) -40.0 40.0)) false false)
    (`KismetSystemLibrary.Delay` 0.001)
    (`self.MoveCamera`)))

(event `InputAxis|Look Up / Down Mouse`
  (params (AxisValue :type "Float (single-precision)"))
  (bind _charref (`self.CharRef`))
  (if (`/Game/FirstPerson/Blueprints/BP_FirstPersonCharacter.isHiding?` _charref)
    (bind _output_get (set `self.pitch` (+ (`self.pitch`) AxisValue)))
    (else
      (`Pawn.AddControllerPitchInput` _charref AxisValue))))

(event `InputAxis|Turn Right / Left Mouse`
  (params (AxisValue :type "Float (single-precision)"))
  (bind _charref (`self.CharRef`))
  (if (`/Game/FirstPerson/Blueprints/BP_FirstPersonCharacter.isHiding?` _charref)
    (bind _output_get (set `self.yaw` (+ (`self.yaw`) AxisValue)))
    (else
      (`Pawn.AddControllerYawInput` _charref AxisValue))))

(fn `UserConstructionScript`)
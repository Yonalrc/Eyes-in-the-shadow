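; Interactive drawer Blueprint that slides open or closed when the player presses the "interagir" input.
; A debug-drawn camera line trace picks any WorldDynamic static mesh component hit, without checking that it belongs to this actor.
; Its relative X against a fixed threshold selects opening or closing, each with a sound and a timeline lerping the position along X.
; An Antispam flag with a delayed reset throttles repeated presses.
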(event `self.ReceiveBeginPlay`
  (`self.EnableInput` (`GameplayStatics.GetPlayerController` 0)))

(event `InputAction|interagir`
  (params (Key :type "Key Structure"))
  (bind _returnvalue (`self.K2_GetActorLocation`))
  (bind (_relativelocation_x _relativelocation_y _relativelocation_z) (`KismetMathLibrary.BreakVector` (`SceneComponent.RelativeLocation` (`self.StaticMeshREF`))))
  (bind (_relativelocation_x_2 _relativelocation_y_2 _relativelocation_z_2) (`KismetMathLibrary.BreakVector` (`SceneComponent.RelativeLocation` (`self.StaticMeshREF`))))
  (:`Pressed`
    (if (not (`self.antispam`))
      (set `self.antispam` true)
      (bind _asbp_first_person_character (cast `/Game/FirstPerson/Blueprints/BP_FirstPersonCharacter` (`GameplayStatics.GetPlayerCharacter` 0)))
      (bind _firstpersoncamera (`/Game/FirstPerson/Blueprints/BP_FirstPersonCharacter.FirstPersonCamera` _asbp_first_person_character))
      (bind _returnvalue_2 (`SceneComponent.K2_GetComponentLocation` _firstpersoncamera))
      (bind (_outhit _returnvalue_3) (`KismetSystemLibrary.LineTraceSingleForObjects` :`Start` _returnvalue_2 :`End` (+ _returnvalue_2 (* (`SceneComponent.GetForwardVector` _firstpersoncamera) 500.0)) :`ObjectTypes` (`|MakeArray` "ObjectTypeQuery2" :!type "EObjectTypeQuery Enum") :`DrawDebugType` "ForDuration" :`bIgnoreSelf` false))
      (if _returnvalue_3
        (bind _asstatic_mesh_component (cast `StaticMeshComponent` (`.HitComponent` (`GameplayStatics.BreakHitResult` _outhit))))
        (set `self.StaticMeshREF` _asstatic_mesh_component)
        (bind _relativelocation_x_3 (`KismetMathLibrary.BreakVector` (`SceneComponent.RelativeLocation` _asstatic_mesh_component)))
        (if (not (>= _relativelocation_x_3 18.0))
          (`GameplayStatics.PlaySoundAtLocation` "/Game/429144__cazadordoblekatana__22-openingdraweramp.429144__cazadordoblekatana__22-openingdraweramp" _returnvalue (struct) 1.0 1.0 0.0 null null null null)
          (set `self.Location Depart` (`KismetMathLibrary.MakeVector` _relativelocation_x _relativelocation_y _relativelocation_z))
          (set `self.Location Arrivé` (`KismetMathLibrary.MakeVector` (+ _relativelocation_x 18.0) _relativelocation_y _relativelocation_z))
          (bind (_direction _ouvrirtiroir) (`Timeline|Ouvrir tiroir` :!via `PlayFromStart`)
            (:`Update`
              (`SceneComponent.K2_SetRelativeLocation` (`self.StaticMeshREF`) (`KismetMathLibrary.VLerp` (`self.Location Depart`) (`self.Location Arrivé`) _ouvrirtiroir) false false)
              (`KismetSystemLibrary.Delay` 1.0)
              (set `self.antispam` false)))
          (else
            (`GameplayStatics.PlaySoundAtLocation` "/Game/538167__leroykhoza__opening-drawer.538167__leroykhoza__opening-drawer" _returnvalue (struct) 1.0 1.0 0.0 null null null null)
            (set `self.Location Depart` (`KismetMathLibrary.MakeVector` _relativelocation_x_2 _relativelocation_y_2 _relativelocation_z_2))
            (set `self.Location Arrivé` (`KismetMathLibrary.MakeVector` (- _relativelocation_x_2 18.0) _relativelocation_y_2 _relativelocation_z_2))
            (bind (_direction_2 _ouvrirtiroir_2) (`Timeline|Timeline` :!via `PlayFromStart`)
              (:`Update`
                (`SceneComponent.K2_SetRelativeLocation` (`self.StaticMeshREF`) (`KismetMathLibrary.VLerp` (`self.Location Depart`) (`self.Location Arrivé`) _ouvrirtiroir_2) false false)
                (`KismetSystemLibrary.Delay` 1.0)
                (set `self.antispam` false)))))
        (else
          (`KismetSystemLibrary.Delay` 1.0)
          (set `self.antispam` false))))))

(fn `UserConstructionScript`)